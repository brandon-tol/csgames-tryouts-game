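; Player-controlled 2D side-scrolling flipbook character with Enhanced Input movement along X and jumping.
; Each tick selects the idle, run, jump or fall flipbook from movement state and turns the controller yaw to face the acceleration direction.
; It also tallies and prints points, and on death calls the game mode's RestartPlayer with self cast to PlayerController, rather than its controller.
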(event Custom|UpdateAnimation
  (bind _charactermovement (Variables|Character|GetCharacterMovement))
  (bind _returnvalue (AI|Components|NavMovement|IsFalling _charactermovement))
  ;[1 1 1] this sets the animation to motion or idle depending on movement or not
  (Sprite|SetFlipbook (Variables|Default|GetSprite) (select (and _returnvalue (> 0.0 (.Z (Class|KismetMathLibrary|BreakVector3f (Variables|/Script/Engine.MovementComponent|GetVelocity (Variables|Character|GetCharacterMovement)))))) "/Game/PNG/sprites/player/jump/FB_P_Fall.FB_P_Fall" (select _returnvalue "/Game/PNG/sprites/player/jump/FB_P_Jump.FB_P_Jump" (select (> (Math|Vector|VectorLength (Variables|/Script/Engine.MovementComponent|GetVelocity (Variables|Character|GetCharacterMovement))) 0.0) "/Game/PNG/sprites/player/run/FB_P_Run.FB_P_Run" "/Game/PNG/sprites/player/idle/FB__P_Idle.FB__P_Idle")))))

(event Custom|UpdateِControlDrection
  ;[1 1 1] this makes the character rotate in the direction it is going
  (Utilities|IsValid (Pawn|GetController)
    (:Is%20Valid
      (Math|Float|CompareFloat (.X (Class|KismetMathLibrary|BreakVector3f (Pawn|Components|CharacterMovement|GetCurrentAcceleration (Variables|Character|GetCharacterMovement)))) 0.0
        (:>
          (Pawn|SetControlRotation (Pawn|GetController) (Math|Rotator|MakeRotator 0.0 0.0 0.0)))
        (:<
          (Pawn|SetControlRotation (Pawn|GetController) (Math|Rotator|MakeRotator 0.0 0.0 1.8e+02)))))))

(event Custom|PlayerDeath
  (Development|PrintString "Player died")
  (Class|GameModeBase|RestartPlayer (Game|GetGameMode) (.AsPlayer%20Controller (Utilities|Casting|CastToPlayerController self))))

(event Custom|AddPoints
  (params (numPoints :type Integer))
  (bind _output_get (Variables|Default|SetTotal%20Points (+ numPoints (Variables|Default|GetTotal%20Points))))
  (Development|PrintString (Utilities|String|Append "Total Points: " (Utilities|String|ToString(Integer) _output_get))))

(event Input|EnhancedActionEvents|EnhancedInputActionIA_Jump
  (params (ActionValue :type Boolean) (ElapsedSeconds :type Float%20%28double-precision%29) (TriggeredSeconds :type Float%20%28double-precision%29) (InputAction :type Input%20Action%20Object%20Reference :default "/Game/Input/Actions/IA_Jump.IA_Jump"))
  ;[1 1 1] Jump calls jump fun
  (:Triggered
    (Character|Jump))
  (:Completed
    (Character|StopJumping)))

(event Input|EnhancedActionEvents|EnhancedInputActionIA_Move
  (params (ActionValue :type Float%20%28double-precision%29) (ElapsedSeconds :type Float%20%28double-precision%29) (TriggeredSeconds :type Float%20%28double-precision%29) (InputAction :type Input%20Action%20Object%20Reference :default "/Game/Input/Actions/IA_Move.IA_Move"))
  ;[1 1 1] Sets movement speed when input
  (:Triggered
    (Pawn|Input|AddMovementInput "1.000000,0.000000,0.000000" (* ActionValue 0.4) false)))

(event EventBeginPlay
  (bind _asplayer_controller (Utilities|Casting|CastToPlayerController (Pawn|GetController)))
  (Input|AddMappingContext (PlayerController|LocalPlayerSubsystems|GetEnhancedInputLocalPlayerSubsystem _asplayer_controller) "/Game/Input/IMC_2D.IMC_2D" 0 "(bIgnoreAllPressedKeysUntilRelease=True,bForceImmediately=False)"))

(event Collision|EventActorBeginOverlap
  (params (OtherActor :type Actor%20Object%20Reference)))

(event EventTick
  (params (DeltaSeconds :type Float%20%28single-precision%29))
  (CallFunction|UpdateAnimation)
  (CallFunction|UpdateِControlDrection))

(fn ConstructionScript)